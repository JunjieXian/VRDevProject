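; VR player character with thumbstick movement and two-handed object gripping, plus mouse look and camera-attached controllers for PC testing.
; Grab input sphere-traces at the controller, picks the highest-priority VRGripInterface target, then makes a primary or secondary grip, using slots when in range.
; Hand socket components supply pose snapshots, mirrored for the left hand, and snap hand meshes onto held objects.
; Dropping restores hand transforms and clears poses.
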(event OnGripOutOfRange(RightMotionController)
  (params (GripInformation :type BP%20Actor%20Grip%20Information%20Structure%20%28by%20ref%29) (Distance :type Float%20%28single-precision%29))
  ;[1 1 1] Grip
  (CallFunction|DropAllGrips (Variables|Default|GetRightMotionController) (Variables|Default|GetLeftMotionController)))

(event Input|EnhancedActionEvents|EnhancedInputActionLeftMotionControllerThumb
  (params (ActionValue :type Vector%202D%20Structure) (ElapsedSeconds :type Float%20%28double-precision%29) (TriggeredSeconds :type Float%20%28double-precision%29) (InputAction :type Input%20Action%20Object%20Reference :default "/Game/MyVRContent/Input/LeftMotionControllerThumb.LeftMotionControllerThumb"))
  ;[1 1 1] Movement
  (:Triggered
    (Pawn|Input|AddMovementInput (Class|VRBaseCharacter|GetVRForwardVector) (.y ActionValue) false)
    (Pawn|Input|AddMovementInput (Class|VRBaseCharacter|GetVRRightVector) (.x ActionValue) false)))

(event Input|EnhancedActionEvents|EnhancedInputActionRightGrab
  (params (ActionValue :type Boolean) (ElapsedSeconds :type Float%20%28double-precision%29) (TriggeredSeconds :type Float%20%28double-precision%29) (InputAction :type Input%20Action%20Object%20Reference :default "/Game/MyVRContent/Input/RightGrab.RightGrab"))
  (bind _leftmotioncontroller (Variables|Default|GetLeftMotionController))
  (bind _rightmotioncontroller (Variables|Default|GetRightMotionController))
  ;[1 1 1] Grip
  (:Started
    (CallFunction|TrytoGripObject _rightmotioncontroller _leftmotioncontroller))
  (:Completed
    (CallFunction|DropAllGrips _rightmotioncontroller _leftmotioncontroller)))

(event Input|EnhancedActionEvents|EnhancedInputActionLeftGrab
  (params (ActionValue :type Boolean) (ElapsedSeconds :type Float%20%28double-precision%29) (TriggeredSeconds :type Float%20%28double-precision%29) (InputAction :type Input%20Action%20Object%20Reference :default "/Game/MyVRContent/Input/LeftGrab.LeftGrab"))
  (bind _rightmotioncontroller (Variables|Default|GetRightMotionController))
  (bind _leftmotioncontroller (Variables|Default|GetLeftMotionController))
  ;[1 1 1] Grip
  (:Started
    (CallFunction|TrytoGripObject _leftmotioncontroller _rightmotioncontroller))
  (:Completed
    (CallFunction|DropAllGrips _leftmotioncontroller _rightmotioncontroller)))

(event Input|EnhancedActionEvents|EnhancedInputActionIA_Mouse
  (params (ActionValue :type Vector%202D%20Structure) (ElapsedSeconds :type Float%20%28double-precision%29) (TriggeredSeconds :type Float%20%28double-precision%29) (InputAction :type Input%20Action%20Object%20Reference :default "/Game/MyVRContent/Input/IA_Mouse.IA_Mouse"))
  ;[1 0 0.01194] PC测试时使用，VR运行需移除
  (:Triggered
    (Pawn|Input|AddControllerPitchInput (* (.y ActionValue) -1.0))
    (Pawn|Input|AddControllerYawInput (.x ActionValue))))

(event EventBeginPlay
  (bind _vrreplicatedcamera (Variables|Default|GetVRReplicatedCamera))
  (Variables|Default|SetDefaultRHandTransform (Transformation|GetRelativeTransform (Variables|Default|GetRightHandSkeletalMesh)))
  (Variables|Default|SetDefaultLHandTransform (Transformation|GetRelativeTransform (Variables|Default|GetLeftHandSkeletalMesh)))
  (Components|Tick|SetTickGroup (Variables|Character|GetMesh) "TG_PostPhysics")
  ;[1 0 0.01194] PC测试时使用，VR运行需移除
  (Transformation|AttachComponentToComponent (Variables|Default|GetLeftMotionController) _vrreplicatedcamera "None" "KeepRelative" "KeepRelative" "KeepRelative" true)
  (Transformation|AttachComponentToComponent (Variables|Default|GetRightMotionController) _vrreplicatedcamera "None" "KeepRelative" "KeepRelative" "KeepRelative" true)
  (Class|ActorComponent|RemoveTickPrerequisiteComponent (Variables|Default|GetLeftMotionController) (Variables|Default|GetVRReplicatedCamera)))

(event Collision|EventActorBeginOverlap
  (params (OtherActor :type Actor%20Object%20Reference)))

(fn ConstructionScript)

(fn TrytoGripObject
  (params (CallingMotionController :type Grip%20Motion%20Controller%20Component%20Object%20Reference) (OtherMotionController :type Grip%20Motion%20Controller%20Component%20Object%20Reference))
  (bind _hand (Class|GripMotionControllerComponent|GetHandType CallingMotionController))
  (bind _hand_2 (Class|GripMotionControllerComponent|GetHandType CallingMotionController))
  (bind _returnvalue (Utilities|Enum|Equal(Enum) _hand_2 "Right"))
  (bind _returnvalue_2 (Utilities|Enum|Equal(Enum) _hand "Right"))
  (if (not (Class|GripMotionControllerComponent|HasGrippedObjects CallingMotionController))
    (bind (_objecttogrip _griplocation _bonename _worldtransform) (CallFunction|GetNearestGripObject CallingMotionController))
    (LocalVariables|SetObjectToGrip _objecttogrip)
    (LocalVariables|SetGripLocation _griplocation)
    (LocalVariables|SetBoneName _bonename)
    (LocalVariables|SetObjectWorldTrasform _worldtransform)
    (bind (_holdingcontrollers _bisheld) (Class|VRGripInterface|IsHeld(Message) (LocalVariables|GetObjectToGrip)))
    (if _bisheld
      (if (CallFunction|CheckSecondaryGrip (LocalVariables|GetObjectToGrip) _holdingcontrollers OtherMotionController)
        (bind (_bhadslotinrange _slotname _transform) (CallFunction|CheckSlotGrip (LocalVariables|GetObjectToGrip) (LocalVariables|GetGripLocation) CallingMotionController (LocalVariables|GetObjectWorldTrasform) (LocalVariables|GetBoneName) true "VRGripS"))
        (Class|GripMotionControllerComponent|AddSecondaryAttachmentPoint OtherMotionController (LocalVariables|GetObjectToGrip) CallingMotionController _transform _bhadslotinrange 0.25 _bhadslotinrange _slotname)
        (CallFunction|HandSlotAttachment (LocalVariables|GetObjectToGrip) (select _returnvalue (Variables|Default|GetRightHandSkeletalMesh) (Variables|Default|GetLeftHandSkeletalMesh)) _slotname _returnvalue) ; 处理手模型的附着，不适用FullBodyIK
        (else
          (bind _returnvalue_3 (Class|VRGripInterface|AllowsMultipleGrips(Message) (LocalVariables|GetObjectToGrip)))
          (if _returnvalue_3
            (bind (_bhadslotinrange_2 _slotname_2 _transform_2) (CallFunction|CheckSlotGrip (LocalVariables|GetObjectToGrip) (LocalVariables|GetGripLocation) CallingMotionController (LocalVariables|GetObjectWorldTrasform) (LocalVariables|GetBoneName) false "VRGripP" :!label _label))
            (Class|GripMotionControllerComponent|GripObjectbyInterface CallingMotionController (LocalVariables|GetObjectToGrip) _transform_2 _bhadslotinrange_2 (LocalVariables|GetBoneName) _slotname_2 _bhadslotinrange_2)
            (CallFunction|HandSlotAttachment (LocalVariables|GetObjectToGrip) (select _returnvalue_2 (Variables|Default|GetRightHandSkeletalMesh) (Variables|Default|GetLeftHandSkeletalMesh)) _slotname_2 _returnvalue_2))))
      (else
        (goto _label)))))

(fn DropAllGrips
  (params (CallingMotionController :type Grip%20Motion%20Controller%20Component%20Object%20Reference) (OtherMotionController :type Grip%20Motion%20Controller%20Component%20Object%20Reference))
  (bind _lefthandskeletalmesh (Variables|Default|GetLeftHandSkeletalMesh))
  (bind _righthandskeletalmesh (Variables|Default|GetRightHandSkeletalMesh))
  (if (Class|GripMotionControllerComponent|HasGrippedObjects CallingMotionController)
    (bind _griparray (Class|GripMotionControllerComponent|GetAllGrips CallingMotionController))
    (for _array_element _griparray
      (Class|GripMotionControllerComponent|DropObjectbyInterface CallingMotionController (.GrippedObject (Utilities|Struct|BreakBPActorGripInformation _array_element)) (.GripID (Utilities|Struct|BreakBPActorGripInformation _array_element)) "0, 0, 0" "0, 0, 0")
      (if (Utilities|Enum|Equal(Enum) (Class|GripMotionControllerComponent|GetHandType CallingMotionController) "Left")
        (Transformation|AttachComponentToComponent _lefthandskeletalmesh CallingMotionController "None" "SnapToTarget" "SnapToTarget" "KeepWorld" true)
        (Transformation|SetRelativeTransform _lefthandskeletalmesh (Variables|Default|GetDefaultLHandTransform) false false)
        (Variables|Default|SetLHandPoseSnap "")
        (else
          (Transformation|AttachComponentToComponent _righthandskeletalmesh CallingMotionController "None" "SnapToTarget" "SnapToTarget" "KeepWorld" true)
          (Transformation|SetRelativeTransform _righthandskeletalmesh (Variables|Default|GetDefaultRHandTransform) false false)
          (Variables|Default|SetRHandPoseSnap ""))))
    (else
      (bind (_grip _returnvalue) (Class|GripMotionControllerComponent|GetIsSecondaryAttachment OtherMotionController CallingMotionController))
      (if _returnvalue
        (Class|GripMotionControllerComponent|RemoveSecondaryAttachmentPoint OtherMotionController (.GrippedObject (Utilities|Struct|BreakBPActorGripInformation _grip)) 0.25)
        (if (Utilities|Enum|Equal(Enum) (Class|GripMotionControllerComponent|GetHandType CallingMotionController) "Left")
          (Transformation|AttachComponentToComponent _lefthandskeletalmesh CallingMotionController "None" "SnapToTarget" "SnapToTarget" "KeepWorld" true)
          (Transformation|SetRelativeTransform _lefthandskeletalmesh (Variables|Default|GetDefaultLHandTransform) false false)
          (Variables|Default|SetLHandPoseSnap "")
          (else
            (Transformation|AttachComponentToComponent _righthandskeletalmesh CallingMotionController "None" "SnapToTarget" "SnapToTarget" "KeepWorld" true)
            (Transformation|SetRelativeTransform _righthandskeletalmesh (Variables|Default|GetDefaultRHandTransform) false false)
            (Variables|Default|SetRHandPoseSnap "")))))))

(fn GetNearestGripObject
  (params (CallingMotionController :type Grip%20Motion%20Controller%20Component%20Object%20Reference))
  (bind _returnvalue (Transformation|GetWorldLocation CallingMotionController))
  (bind (_outhits _returnvalue_2) (Collision|MultiSphereTraceByChannel _returnvalue _returnvalue 5.0 "TraceTypeQuery1" false 0 "ForDuration"))
  (if _returnvalue_2
    (bind (_objecttogrip _griplocation _bonename _worldtransform) (CallFunction|SelectGripObjectfromHits _outhits CallingMotionController))
    (Utilities|IsValid _objecttogrip
      (:Is%20Valid
        (return _objecttogrip _griplocation _bonename _worldtransform))
      (:Is%20Not%20Valid
        _)))
  (return 0 "0, 0, 0" "None" ""))

(fn SelectGripObjectfromHits
  (params (HitObjects :type Array%20of%20Hit%20Result%20Structures) (GripInitiator :type Grip%20Motion%20Controller%20Component%20Object%20Reference))
  (for _array_element HitObjects
    (bind (_isbestprio _newgrippriority _newobject _hitlocation _hitbonename _worldtransform) (CallFunction|CheckBestGripObject _array_element (LocalVariables|GetBestGripPrio) GripInitiator))
    (if _isbestprio
      (LocalVariables|SetBestGripPrio _newgrippriority)
      (LocalVariables|SetLObjectToGrip _newobject)
      (LocalVariables|SetLGripLocation _hitlocation)
      (LocalVariables|SetLBoneName _hitbonename)
      (LocalVariables|SetLWorldTransform _worldtransform)))
  (return (LocalVariables|GetLObjectToGrip) (LocalVariables|GetLGripLocation) (LocalVariables|GetLBoneName) (LocalVariables|GetLWorldTransform)))

(fn CheckBestGripObject
  (params (HitObject :type Hit%20Result%20Structure) (DefaultPriority :type Byte) (GripInitiator :type Grip%20Motion%20Controller%20Component%20Object%20Reference))
  (bind (_bblockinghit _binitialoverlap _time _distance _location _impactpoint _normal _impactnormal _physmat _hitactor _hitcomponent _hitbonename) (Collision|BreakHitResult HitObject))
  (if (Utilities|DoesObjectImplementInterface _hitcomponent "/Script/VRExpansionPlugin.VRGripInterface")
    (bind _returnvalue (Class|VRGripInterface|DenyGripping(Message) _hitcomponent GripInitiator))
    (if _returnvalue
      _
      (else
        (bind _returnvalue_2 (Class|VRGripInterface|AdvancedGripSettings(Message) _hitcomponent))
        (if (> (.grippriority _returnvalue_2) DefaultPriority)
          (return true (.grippriority _returnvalue_2) _hitcomponent _location _hitbonename (Transformation|GetWorldTransform _hitcomponent))
          (else
            _))))
    (elif (Utilities|DoesObjectImplementInterface _hitactor "/Script/VRExpansionPlugin.VRGripInterface")
      (bind _returnvalue_3 (Class|VRGripInterface|DenyGripping(Message) _hitactor GripInitiator))
      (if _returnvalue_3
        _
        (else
          (bind _returnvalue_4 (Class|VRGripInterface|AdvancedGripSettings(Message) _hitactor))
          (if (> (.grippriority _returnvalue_4) DefaultPriority)
            (return true (.grippriority _returnvalue_4) _hitactor _location _hitbonename (Transformation|GetActorTransform _hitactor))
            (else
              _))))))
  (return false 0 0 "0, 0, 0" "None" ""))

(fn CheckBoneWorldTransform
  (params (ObjectToCheck :type Object%20Object%20Reference) (BoneName :type Name) (WorldTransform :type Transform))
  (if (!= BoneName "")
    (bind _asskeletal_mesh_component (Utilities|Casting|CastToSkeletalMeshComponent ObjectToCheck)
      (:then
        (return (Transformation|GetSocketTransform _asskeletal_mesh_component BoneName "RTS_World")))
      (:CastFailed
        (bind _asskeletal_mesh_actor (Utilities|Casting|CastToSkeletalMeshActor ObjectToCheck)
          (:then
            (return (Transformation|GetSocketTransform (Variables|/Script/Engine.SkeletalMeshActor|GetSkeletalMeshComponent _asskeletal_mesh_actor) BoneName "RTS_World")))
          (:CastFailed
            _)))))
  (return WorldTransform))

(fn CheckSlotGrip
  (params (ObjectToCheck :type Object%20Object%20Reference) (WorldLocation :type Vector) (CallingController :type Grip%20Motion%20Controller%20Component%20Object%20Reference) (WorldTransform :type Transform) (BoneName :type Name) (bSecondarySlot :type Boolean) (OverridePrefix :type Name))
  (bind _transform (CallFunction|CheckBoneWorldTransform ObjectToCheck BoneName WorldTransform))
  (bind _hand (Class|GripMotionControllerComponent|GetHandType CallingController))
  (bind _returnvalue (Utilities|Enum|Equal(Enum) _hand "Left"))
  (bind (_bhadslotinrange _slotworldtransform _slotname) (Class|VRGripInterface|ClosestGripSlotinRange(Message) ObjectToCheck WorldLocation bSecondarySlot CallingController OverridePrefix))
  (if _bhadslotinrange
    ;[0.0349 0.4746 1] HandPose
    (bind _returnvalue_2 (Class|HandSocketComponent|GetHandSocketComponentfromObject ObjectToCheck _slotname))
    (Utilities|IsValid _returnvalue_2
      (:Is%20Valid
        (bind _posesnapshot (Class|HandSocketComponent|GetBlendedPoseSnapShot _returnvalue_2 (Variables|Character|GetMesh) false _returnvalue))
        (if _returnvalue
          (Variables|Default|SetLHandPoseSnap _posesnapshot)
          (else
            (Variables|Default|SetRHandPoseSnap _posesnapshot))))
      (:Is%20Not%20Valid
        _)))
  (return _bhadslotinrange _slotname (Math|Transform|SelectTransform (select bSecondarySlot (Class|GripMotionControllerComponent|ConverttoGripRelativeTransform _transform _slotworldtransform) (Class|KismetMathLibrary|ConvertTransformtoRelative _slotworldtransform _transform)) _transform _bhadslotinrange)))

(fn CheckSecondaryGrip
  (params (ObjectToCheck :type Object%20Object%20Reference) (HoldingControllers :type Array%20of%20BP%20Grip%20Pair%20Structures) (OtherMotionController :type Object%20Object%20Reference))
  (bind _returnvalue (Class|VRGripInterface|SecondaryGripType(Message) ObjectToCheck))
  (return (and (Utilities|Enum|NotEqual(Enum) _returnvalue "SG_None") (== (.holdingcontroller (Utilities|Array|Get(acopy) HoldingControllers)) OtherMotionController))))

(fn HandSlotAttachment
  (params (ObjectToAttachment :type Object%20Object%20Reference) (HandSkeletalMesh :type Skeletal%20Mesh%20Component%20Object%20Reference) (SlotName :type Name) (bIsRightHand :type Boolean))
  (bind _returnvalue (Class|HandSocketComponent|GetHandSocketComponentfromObject ObjectToAttachment SlotName))
  (Utilities|IsValid _returnvalue
    (:Is%20Valid
      (bind _returnvalue_2 (Class|HandSocketComponent|GetMeshRelativeTransform _returnvalue bIsRightHand false false))
      (LocalVariables|SetMeshRelativeTransform _returnvalue_2)
      (bind _asprimitive_component (Utilities|Casting|CastToPrimitiveComponent ObjectToAttachment)
        (:then
          (Transformation|AttachComponentToComponent HandSkeletalMesh _asprimitive_component "None" "SnapToTarget" "SnapToTarget" "KeepWorld" true))
        (:CastFailed
          (bind _asactor (Utilities|Casting|CastToActor ObjectToAttachment))
          (Transformation|AttachComponentToComponent HandSkeletalMesh (Variables|/Script/Engine.Actor|GetRootComponent _asactor) "None" "SnapToTarget" "SnapToTarget" "KeepWorld" true)))
      (Transformation|SetRelativeLocationAndRotation HandSkeletalMesh (.location (LocalVariables|GetMeshRelativeTransform)) (.rotation (LocalVariables|GetMeshRelativeTransform)) false false)
      (Transformation|SetWorldScale3D HandSkeletalMesh (.scale (LocalVariables|GetMeshRelativeTransform))))))